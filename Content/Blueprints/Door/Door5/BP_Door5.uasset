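; BP_Door5 is a sliding double door that alternates between opening and closing on each OpenDoor call.
; A FlipFlop plays or reverses a Timeline, which slides LeftDoor5 and RightDoor5 apart on local Y by mirrored Lerp offsets.
; OpenDoor also prints a debug string.
; The Interact event reads the player's code-correct message, but its branch does nothing and never calls OpenDoor.
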(event `/Game/Blueprints/Door/Door5/Keypad/BPI_InteractionKeypad.E-Interact`
  ;[1 1 1] Mécanisme (+ animation) d'ouverture et de fermeture de la porte
  (bind _unlocked_ (message `/Game/Blueprints/Door/Door5/Keypad/BPI_UnlockDoor.Get code correct` (`GameplayStatics.GetPlayerCharacter` 0)))
  (if _unlocked_
    _))

(event `OpenDoor`
  ;[1 1 1] Mécanisme (+ animation) d'ouverture et de fermeture de la porte
  (`KismetSystemLibrary.PrintString` "PORTE RECUE")
  (`/Engine/EditorBlueprintResources/StandardMacros.FlipFlop`
    (:`A`
      (bind (_direction _alpha) (`Timeline|Timeline` :!label _label)
        (:`Update`
          (bind _returnvalue (`KismetMathLibrary.Lerp` 0.0 150.0 _alpha))
          (`SceneComponent.K2_SetRelativeLocation` (`self.LeftDoor5`) (`KismetMathLibrary.MakeVector` 0.0 _returnvalue) false false)
          (`SceneComponent.K2_SetRelativeLocation` (`self.RightDoor5`) (`KismetMathLibrary.MakeVector` 0.0 (* _returnvalue -1.0)) false false))))
    (:`B`
      (goto _label :!via `Reverse`))))

(fn `UserConstructionScript`)