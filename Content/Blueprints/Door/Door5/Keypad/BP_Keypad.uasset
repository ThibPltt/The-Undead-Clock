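; BP_Keypad is an interactive in-world keypad that opens Door5 when the correct code is entered.
; E-Interact blends the view to the keypad, locks player look and movement, and enables mouse clicks.
; Clickable buttons feed Code, which updates the WBP_Keypad display, checks the code and clears at five digits.
; A match opens the door, turns KeypadSpheres green and restores player control, which Q also does through Exit.
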(event `self.ReceiveBeginPlay`
  ;[1 1 1] Apparition du widget Keypad
  (bind _aswbp_keypad (cast `/Game/Blueprints/Door/Door5/Keypad/WBP_Keypad` (`WidgetComponent.GetWidget` (`self.Widget`))))
  (set `self.As WBP Keypad` _aswbp_keypad))

(event `/Game/Blueprints/Door/Door5/Keypad/BPI_InteractionKeypad.E-Interact`
  (bind _returnvalue (`GameplayStatics.GetPlayerController` 0))
  (bind _returnvalue_2 (`GameplayStatics.GetPlayerController` 0))
  ;[1 1 1] Fonctionnement de l'interaction avec le Keypad une fois la vue fixée dessus
  (`PlayerController.SetViewTargetWithBlend` _returnvalue_2 self 0.3 "VTBlend_Linear" 0.0 false)
  (`Controller.SetIgnoreLookInput` _returnvalue_2 true)
  (set `PlayerController.bEnableClickEvents` true _returnvalue_2)
  (set `PlayerController.bShowMouseCursor` true _returnvalue_2)
  (`CharacterMovementComponent.DisableMovement` (`Character.CharacterMovement` (`GameplayStatics.GetPlayerCharacter` 0)))
  (`self.EnableInput` _returnvalue)
  (`WidgetBlueprintLibrary.SetInputMode_GameAndUIEx` _returnvalue null))

(event `self.Keypad_button1.OnClicked`
  (params (TouchedComponent :type "PrimitiveComponent Object Reference") (ButtonPressed :type "Key Structure"))
  ;[1 1 1] Interactions avec les boutons
  (`self.Code` "1"))

(event `Key|Q`
  (params (Key :type "Key Structure"))
  (bind _returnvalue (`GameplayStatics.GetPlayerController` 0))
  (:`Pressed`
    (`PlayerController.SetViewTargetWithBlend` _returnvalue (`GameplayStatics.GetPlayerCharacter` 0) 0.3 "VTBlend_Linear" 0.0 false)
    (`Controller.ResetIgnoreLookInput` _returnvalue)
    (set `PlayerController.bEnableClickEvents` false _returnvalue)
    (set `PlayerController.bShowMouseCursor` false _returnvalue)
    (`CharacterMovementComponent.SetMovementMode` (`Character.CharacterMovement` (`GameplayStatics.GetPlayerCharacter` 0)) "MOVE_Walking" 0)
    (`WidgetBlueprintLibrary.SetInputMode_GameOnly` _returnvalue)
    (`self.DisableInput` _returnvalue)))

(event `self.Keypad_button2.OnClicked`
  (params (TouchedComponent :type "PrimitiveComponent Object Reference") (ButtonPressed :type "Key Structure"))
  ;[1 1 1] Interactions avec les boutons
  (`self.Code` "2"))

(event `self.Keypad_button3.OnClicked`
  (params (TouchedComponent :type "PrimitiveComponent Object Reference") (ButtonPressed :type "Key Structure"))
  ;[1 1 1] Interactions avec les boutons
  (`self.Code` "3"))

(event `self.Keypad_button4.OnClicked`
  (params (TouchedComponent :type "PrimitiveComponent Object Reference") (ButtonPressed :type "Key Structure"))
  ;[1 1 1] Interactions avec les boutons
  (`self.Code` "4"))

(event `self.Keypad_button5.OnClicked`
  (params (TouchedComponent :type "PrimitiveComponent Object Reference") (ButtonPressed :type "Key Structure"))
  ;[1 1 1] Interactions avec les boutons
  (`self.Code` "5"))

(event `self.Keypad_button6.OnClicked`
  (params (TouchedComponent :type "PrimitiveComponent Object Reference") (ButtonPressed :type "Key Structure"))
  ;[1 1 1] Interactions avec les boutons
  (`self.Code` "6"))

(event `self.Keypad_button7.OnClicked`
  (params (TouchedComponent :type "PrimitiveComponent Object Reference") (ButtonPressed :type "Key Structure"))
  ;[1 1 1] Interactions avec les boutons
  (`self.Code` "7"))

(event `self.Keypad_button8.OnClicked`
  (params (TouchedComponent :type "PrimitiveComponent Object Reference") (ButtonPressed :type "Key Structure"))
  ;[1 1 1] Interactions avec les boutons
  (`self.Code` "8"))

(event `self.Keypad_button9.OnClicked`
  (params (TouchedComponent :type "PrimitiveComponent Object Reference") (ButtonPressed :type "Key Structure"))
  ;[1 1 1] Interactions avec les boutons
  (`self.Code` "9"))

(event `self.Keypad_button0.OnClicked`
  (params (TouchedComponent :type "PrimitiveComponent Object Reference") (ButtonPressed :type "Key Structure"))
  ;[1 1 1] Interactions avec les boutons
  (`self.Code` "0"))

(fn `Code`
  (params (B :type String))
  (bind _returnvalue (`GameplayStatics.GetPlayerController` 0))
  (bind _returnvalue_2 (`GameplayStatics.GetPlayerCharacter` 0))
  (`GameplayStatics.PlaySound2D` "/Game/Blueprints/Door/Door5/Keypad/key_code_sfx.key_code_sfx" 1.0 1.0 0.0 null null)
  (bind _output_get (set `self.Input` (`KismetStringLibrary.Concat_StrStr` (`self.Input`) B)))
  (set `self.Length of Code` (+ (`self.Length of Code`) 1))
  (`TextBlock.SetText` (`/Game/Blueprints/Door/Door5/Keypad/WBP_Keypad.CodeText` (`self.As WBP Keypad`)) (`KismetTextLibrary.Conv_StringToText` _output_get))
  (if (`KismetStringLibrary.EqualEqual_StrStr` (`self.Input`) (`self.Correct Code`))
    (`KismetSystemLibrary.PrintString` "keypad ok")
    (`/Game/Blueprints/Door/Door5/BP_Door5.OpenDoor` (`self.Door5`))
    (message `/Game/Blueprints/Door/Door5/Keypad/BPI_UnlockDoor.Set code correct` (`GameplayStatics.GetPlayerCharacter` 0) true)
    (`PrimitiveComponent.SetMaterial` (`self.Keypad_spheres`) 0 "/Game/Blueprints/Door/Door5/Keypad/MI_KGreen.MI_KGreen")
    (`self.DisableInput` _returnvalue)
    (`PlayerController.SetViewTargetWithBlend` _returnvalue _returnvalue_2 0.3 "VTBlend_Linear" 0.0 false)
    (`Controller.ResetIgnoreLookInput` _returnvalue)
    (set `PlayerController.bEnableClickEvents` false _returnvalue)
    (set `PlayerController.bShowMouseCursor` false _returnvalue)
    (`CharacterMovementComponent.SetMovementMode` (`Character.CharacterMovement` _returnvalue_2) "MOVE_Walking" 0)
    (`WidgetBlueprintLibrary.SetInputMode_GameOnly` _returnvalue))
  (if (>= (`self.Length of Code`) 5)
    (bind _output_get_2 (set `self.Input` ""))
    (`TextBlock.SetText` (`/Game/Blueprints/Door/Door5/Keypad/WBP_Keypad.CodeText` (`self.As WBP Keypad`)) (`KismetTextLibrary.Conv_StringToText` _output_get_2))
    (set `self.Length of Code` 0)))

(fn `UserConstructionScript`)