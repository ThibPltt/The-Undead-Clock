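; BP_ButtonFinal4 is an interactable button that opens and closes Door4 once the wave number in BP_FirstPersonGameMode is above 8.
; When unlocked, a FlipFlop alternates each interaction between OpenDoor4 and CloseDoor4 on the door.
; While locked, it briefly shows a WBP_MessageButton widget asking to finish wave 8, with a DoOnce reset after removal to prevent stacked messages.
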(event `/Game/Blueprints/Door/Door1/BPI_Interaction2.Interact`
  (bind _door4 (`self.Door4`))
  ;[1 1 1] Bouton activable seulement après la vague 2
  (bind _asbp_first_person_game_mode (cast `/Game/FirstPerson/Blueprints/BP_FirstPersonGameMode` (`GameplayStatics.GetGameMode`)))
  ;[1 1 1] Ouverture/Fermeture de la porte en appuyant sur le bouton (et message de verrouillage si vague < 2)
  (if (> (`/Game/FirstPerson/Blueprints/BP_FirstPersonGameMode.WaveNumber` _asbp_first_person_game_mode) 8)
    (`/Engine/EditorBlueprintResources/StandardMacros.FlipFlop`
      (:`A`
        (`/Game/Blueprints/Door/Door4/BP_Door4.OpenDoor4` _door4))
      (:`B`
        (`/Game/Blueprints/Door/Door4/BP_Door4.CloseDoor4` _door4)))
    (else
      (`/Engine/EditorBlueprintResources/StandardMacros.DoOnce` false :!label _label
        (:`Completed`
          (bind _returnvalue (`|CreateWidget` "/Game/FirstPerson/Widget/WBP_MessageButton.WBP_MessageButton_C" null "Finir Vague 8"))
          (`UserWidget.AddToViewport` _returnvalue 0)
          (`KismetSystemLibrary.Delay` 2.0)
          (`Widget.RemoveFromParent` _returnvalue)
          (goto _label :!via `Reset`))))))

(fn `UserConstructionScript`)