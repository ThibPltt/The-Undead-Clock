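; Base Blueprint for full-auto weapons that keep firing from Shoot until EndShoot, extending a parent weapon class.
; Shoot calls the parent, then starts a looping timer at the FireRate interval that runs a shot trace over Range on each tick.
; EndShoot calls the parent and clears the timer handle to stop the fire loop.
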(event `self.Shoot`
  ;[1 1 1] Mécanisme de shoot
  (`parent.Shoot`)
  (bind _returnvalue (`KismetSystemLibrary.K2_SetTimerDelegate` (delegate `FullAutoShoot`) (`self.FireRate`) true))
  (set `self.Timer` _returnvalue))

(event `FullAutoShoot`
  ;[1 1 1] Mécanisme de shoot
  (`self.CreateShotTrace` (`self.Range`)))

(event `self.EndShoot`
  ;[1 1 1] Mécanisme de shoot
  (`parent.EndShoot`)
  (`KismetSystemLibrary.K2_ClearAndInvalidateTimerHandle` (`self.Timer`)))

(fn `UserConstructionScript`
  (`parent.UserConstructionScript`))