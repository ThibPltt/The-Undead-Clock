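; BP_BaseSemiAutoWeapon is a base semi-automatic weapon that adds a delay between shots.
; Shoot calls the parent implementation, then, if CanShoot is true, clears that flag and creates a shot trace over Range.
; A non-looping timer restores CanShoot through ResetShot after FireRate, so FireRate acts as an interval in seconds.
; The parent Shoot runs on every call, even during the cooldown.
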(event `self.Shoot`
  ;[1 1 1] Ajout d'un délais pour tirer
  (`parent.Shoot`)
  (if (`self.CanShoot?`)
    (set `self.CanShoot?` false)
    (`self.CreateShotTrace` (`self.Range`))
    (`KismetSystemLibrary.K2_SetTimerDelegate` (delegate `ResetShot`) (`self.FireRate`))))

(event `ResetShot`
  ;[1 1 1] Ajout d'un délais pour tirer
  (set `self.CanShoot?` true))

(fn `UserConstructionScript`
  (`parent.UserConstructionScript`))