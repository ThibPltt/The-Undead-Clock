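; Base weapon Blueprint that provides hitscan shot tracing, damage and impact effects, with empty Shoot and EndShoot events.
; CreateShotTrace spawns a muzzle effect on ShotArrow, then multi-traces forward over the given range against pawns and static world objects.
; Every hit actor takes damage and spawns particles chosen by its first actor tag, with glass, zombie blood or a ceramic default.
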(event `EndShoot`)

(event `Shoot`)

(event `CreateShotTrace`
  (params (Range :type "Float (double-precision)"))
  (bind _shotarrow (`self.ShotArrow`))
  (bind _returnvalue (`SceneComponent.K2_GetComponentLocation` _shotarrow))
  (bind _returnvalue_2 (`SceneComponent.K2_GetComponentRotation` _shotarrow))
  (`GameplayStatics.SpawnEmitterAttached` "/Game/Realistic_Starter_VFX_Pack_Vol2/Particles/Explosion/P_Explosion_Big_A.P_Explosion_Big_A" _shotarrow "None" (0.0 0.0 0.0) (struct) (0.03 0.03 0.03))
  (bind (_outhits _returnvalue_3) (`KismetSystemLibrary.LineTraceMultiForObjects` _returnvalue (+ _returnvalue (* (`KismetMathLibrary.GetForwardVector` _returnvalue_2) Range)) (`|MakeArray` "ObjectTypeQuery3" "ObjectTypeQuery1" :!type "EObjectTypeQuery Enum")))
  (if _returnvalue_3
    (for _array_element _outhits
      (bind (_bblockinghit _binitialoverlap _time _distance _location _impactpoint _normal _impactnormal _physmat _hitactor) (`GameplayStatics.BreakHitResult` _array_element))
      ;[1 1 1] Particules sur chaque objet quand on tire
      (`self.SpawnHitParticles` (`|GetArrayItem` (`Actor.Tags` _hitactor)) _location _returnvalue_2)
      (`GameplayStatics.ApplyDamage` _hitactor (`self.Damage`)))))

(event `SpawnHitParticles`
  (params (TagName :type Name) (Location :type "Vector Structure") (ArrowRotation :type "Rotator Structure"))
  ;[1 1 1] Différentiation des particules selon le matériau touché
  (switch `name` TagName
    (:`Default`
      (set `self.HitsParticles` "/Game/Realistic_Starter_VFX_Pack_Vol2/Particles/Hit/P_Ceramic.P_Ceramic"))
    (:`Glass`
      (set `self.HitsParticles` "/Game/Realistic_Starter_VFX_Pack_Vol2/Particles/Destruction/P_Destruction_Glass.P_Destruction_Glass"))
    (:`Zombie`
      (set `self.HitsParticles` "/Game/Realistic_Starter_VFX_Pack_Vol2/Particles/Blood/P_Blood_Splat_Cone.P_Blood_Splat_Cone")))
  (`GameplayStatics.SpawnEmitterAtLocation` (`self.HitsParticles`) Location (`KismetMathLibrary.MakeRotator` (.roll ArrowRotation) (+ (.pitch ArrowRotation) 120.0) (.yaw ArrowRotation)) (0.4 0.4 0.4)))

(fn `UserConstructionScript`)