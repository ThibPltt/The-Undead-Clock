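; Behavior Tree service that lets zombie AI detect the player within a search radius.
; On each tick it runs a multi sphere trace for Pawn objects at the controlled pawn's location, sized by the SearchRadius blackboard key, with timed debug drawing.
; A hit that casts to BP_FirstPersonCharacter is written to the TargetCharacter key, which is cleared when no player is found.
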(event `self.ReceiveTickAI`
  (params (OwnerController :type "AIController Object Reference") (ControlledPawn :type "Pawn Object Reference") (DeltaSeconds :type "Float (single-precision)"))
  (bind _returnvalue (`Actor.K2_GetActorLocation` ControlledPawn))
  (bind _playercharacter (`self.PlayerCharacter`))
  (bind _targetcharacter (`self.TargetCharacter`))
  ;[1 1 1] Déplacements aléatoires des zombies
  (set `self.PlayerCharacter` null)
  (bind (_outhits _returnvalue_2) (`KismetSystemLibrary.SphereTraceMultiForObjects` :`Start` _returnvalue :`End` _returnvalue :`Radius` (`BTFunctionLibrary.GetBlackboardValueAsFloat` (`self.SearchRadius`)) :`ObjectTypes` (`|MakeArray` "ObjectTypeQuery3" :!type "EObjectTypeQuery Enum") :`DrawDebugType` "ForDuration"))
  (if _returnvalue_2
    (for _array_element _outhits
      (bind _asbp_first_person_character (cast `/Game/FirstPerson/Blueprints/BP_FirstPersonCharacter` (`.HitActor` (`GameplayStatics.BreakHitResult` _array_element))))
      (set `self.PlayerCharacter` _asbp_first_person_character)))
  (`/Engine/EditorBlueprintResources/StandardMacros.IsValid` _playercharacter
    (:`Is Valid`
      (`BTFunctionLibrary.SetBlackboardValueAsObject` _targetcharacter _playercharacter))
    (:`Is Not Valid`
      (`BTFunctionLibrary.ClearBlackboardValue` _targetcharacter))))