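; BP_WallLight is an interactable wall light that the MainInteraction event toggles on and off.
; Each toggle flips the On state and calls LightEvent, optionally playing a sound at the actor's location when switching on.
; LightEvent, also run on BeginPlay to apply the initial state, drives both the mesh material's Glow parameter and the point light's intensity from that state.
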(event `self.ReceiveBeginPlay`
  (`parent.ReceiveBeginPlay`)
  (`self.LightEvent`))

(event `/Game/SmartBasicInterfaces/Blueprints/BP_MasterInteractable.MainInteraction`
  (if (`self.On`)
    (set `self.On` false)
    (else
      (set `self.On` true)
      (if (`self.PlaySound`)
        (`GameplayStatics.PlaySoundAtLocation` "/Game/SmartBasicInterfaces/Sound/SC_lighton.SC_lighton" (`self.K2_GetActorLocation`) (struct) 1.0 1.0 0.0 null null null null))))
  (`self.LightEvent`))

(event `LightEvent`
  (`MeshComponent.SetScalarParameterValueOnMaterials` (`self.Light`) "Glow" (`KismetMathLibrary.SelectFloat` 5.0 0.0 (`self.On`)))
  (`LightComponent.SetIntensity` (`self.PointLight`) (`KismetMathLibrary.SelectFloat` 5000.0 0.0 (`self.On`))))

(fn `UserConstructionScript`
  (`parent.UserConstructionScript`))