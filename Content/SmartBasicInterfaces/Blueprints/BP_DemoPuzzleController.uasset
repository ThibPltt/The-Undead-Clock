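; Demo-only controller for the L_Demo puzzle level that tracks objectives in a WI_DemoTracker widget and links the puzzle actors together.
; On BeginPlay it binds to events from buttons, a trip laser, doors, generator and panel, most setting tracker flags.
; Fuel triggers the generator if the lever is on, generator power drives the panel, and a full card set activates the pressure plate.
; Fully opened doors show the demo-over widget.
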(event `LevelEnd`
  ;[1 1 1] This Blueprint Is Only relevelant for the L_Demo. You can safely ignore it for your project
  (bind _returnvalue (`|CreateWidget` "/Game/SmartBasicInterfaces/Widgets/WI_DemoOver.WI_DemoOver_C"))
  (`UserWidget.AddToViewport` _returnvalue 0))

(event `Set Q4`
  ;[1 1 1] This Blueprint Is Only relevelant for the L_Demo. You can safely ignore it for your project
  (set `/Game/SmartBasicInterfaces/Widgets/WI_DemoTracker.bQ_4` true (`self.TrackerUI`)))

(event `Set Q8`
  ;[1 1 1] This Blueprint Is Only relevelant for the L_Demo. You can safely ignore it for your project
  (set `/Game/SmartBasicInterfaces/Widgets/WI_DemoTracker.bQ_8` true (`self.TrackerUI`)))

(event `AllowPressurePlate`
  ;[1 1 1] This Blueprint Is Only relevelant for the L_Demo. You can safely ignore it for your project
  (set `/Game/SmartBasicInterfaces/Blueprints/BP_MasterControl.Active` true (`self.PressurePlate`))
  (set `/Game/SmartBasicInterfaces/Widgets/WI_DemoTracker.bQ_9` true (`self.TrackerUI`)))

(event `Set Q5`
  ;[1 1 1] This Blueprint Is Only relevelant for the L_Demo. You can safely ignore it for your project
  (set `/Game/SmartBasicInterfaces/Widgets/WI_DemoTracker.bQ_5` true (`self.TrackerUI`)))

(event `Set Q2`
  ;[1 1 1] This Blueprint Is Only relevelant for the L_Demo. You can safely ignore it for your project
  (set `/Game/SmartBasicInterfaces/Widgets/WI_DemoTracker.bQ_2` true (`self.TrackerUI`)))

(event `Set Q1`
  ;[1 1 1] This Blueprint Is Only relevelant for the L_Demo. You can safely ignore it for your project
  (set `/Game/SmartBasicInterfaces/Widgets/WI_DemoTracker.bQ_1` true (`self.TrackerUI`)))

(event `Set Q3`
  ;[1 1 1] This Blueprint Is Only relevelant for the L_Demo. You can safely ignore it for your project
  (set `/Game/SmartBasicInterfaces/Widgets/WI_DemoTracker.bQ_3` true (`self.TrackerUI`)))

(event `self.ReceiveBeginPlay`
  ;[1 1 1] This Blueprint Is Only relevelant for the L_Demo. You can safely ignore it for your project
  (`parent.ReceiveBeginPlay`)
  (bind _returnvalue (`|CreateWidget` "/Game/SmartBasicInterfaces/Widgets/WI_DemoTracker.WI_DemoTracker_C"))
  (bind _output_get (set `self.TrackerUI` _returnvalue))
  (`UserWidget.AddToViewport` _output_get 0)
  (add `/Game/SmartBasicInterfaces/Blueprints/BP_Generator.GeneratorOn` (`self.Generator`) (delegate `CheckGenertor`))
  (add `/Game/SmartBasicInterfaces/Blueprints/BP_AccessPanel.PanelWithAllCards` (`self.Panel`) (delegate `AllowPressurePlate`))
  (add `/Game/SmartBasicInterfaces/Blueprints/BP_Generator.HasFuel` (`self.Generator`) (delegate `CheckIfLeverIsOn`))
  (add `/Game/SmartBasicInterfaces/Blueprints/BP_DoubleDoor.DoorFullyOpen` (`self.Doors`) (delegate `LevelEnd`))
  (add `/Game/SmartBasicInterfaces/Blueprints/BP_PowerBTN.ButtonPressed` (`self.StartBTN`) (delegate `Set Q1`))
  (add `/Game/SmartBasicInterfaces/Blueprints/BP_PowerBTN.ButtonPressed` (`self.AlarmBTN`) (delegate `Set Q3`))
  (bind _outactors (`GameplayStatics.GetAllActorsOfClass` "/Game/SmartBasicInterfaces/Blueprints/BP_TripLaser.BP_TripLaser_C"))
  (add `/Game/SmartBasicInterfaces/Blueprints/BP_TripLaser.TripWireActive` (`|GetArrayItem` _outactors) (delegate `Set Q2`))
  (add `/Game/SmartBasicInterfaces/Blueprints/BP_SimpleDoor.DoorControl` (`self.CorridorDoor`) (delegate `Set Q5`)))

(event `CheckGenertor`
  (bind _panel (`self.Panel`))
  ;[1 1 1] This Blueprint Is Only relevelant for the L_Demo. You can safely ignore it for your project
  (set `/Game/SmartBasicInterfaces/Blueprints/BP_MasterControl.Active` (`/Game/SmartBasicInterfaces/Blueprints/BP_MasterInteractable.TurnedOn` (`self.Generator`)) _panel)
  (set `/Game/SmartBasicInterfaces/Widgets/WI_DemoTracker.bQ_7` true (`self.TrackerUI`))
  (`/Game/SmartBasicInterfaces/Blueprints/BP_AccessPanel.Visibility` _panel))

(event `CheckIfLeverIsOn`
  ;[1 1 1] This Blueprint Is Only relevelant for the L_Demo. You can safely ignore it for your project
  (set `/Game/SmartBasicInterfaces/Widgets/WI_DemoTracker.bQ_6` true (`self.TrackerUI`))
  (if (`/Game/SmartBasicInterfaces/Blueprints/BP_MasterInteractable.TurnedOn` (`self.Lever`))
    (`/Game/SmartBasicInterfaces/Blueprints/BP_MasterInteractable.MainInteraction` (`self.Generator`))))

(fn `UserConstructionScript`)