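; BP_TimerDisplay is a demo actor for L_QuickDemo that shows a countdown as in-world text.
; On BeginPlay, FindNearest searches all BP_MasterControl actors and stores the closest one within the initial Default distance as Control.
; Every tick, it writes the remaining time of that control's DelayTH timer to its TextRender, or "On Stand By" when no time remains.
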(event `self.ReceiveBeginPlay`
  ;[1 1 1] Actor for L_QuickDemo. Just a timer display
  (`parent.ReceiveBeginPlay`)
  (`self.FindNearest`))

(event `self.ReceiveTick`
  (params (DeltaSeconds :type "Float (single-precision)"))
  ;[1 1 1] Actor for L_QuickDemo. Just a timer display
  (`parent.ReceiveTick` DeltaSeconds)
  (`self.Set Text`))

(event `Set Text`
  (bind _returnvalue (`KismetSystemLibrary.K2_GetTimerRemainingTimeHandle` (`/Game/SmartBasicInterfaces/Blueprints/BP_MasterControl.DelayTH` (`self.Control`))))
  ;[1 1 1] Actor for L_QuickDemo. Just a timer display
  (if (<= _returnvalue 0.0)
    (`TextRenderComponent.K2_SetText` (`self.TextRender`) "On Stand By")
    (else
      (`TextRenderComponent.K2_SetText` (`self.TextRender`) (`KismetTextLibrary.Conv_DoubleToText` _returnvalue "HalfToEven")))))

(fn `FindNearest`
  (locals (Default :type "Float (double-precision)" :default 10000.0) (Nearest :type "/Game/SmartBasicInterfaces/Blueprints/BP_MasterControl Object Reference"))
  (bind _outactors (`GameplayStatics.GetAllActorsOfClass` "/Game/SmartBasicInterfaces/Blueprints/BP_MasterControl.BP_MasterControl_C"))
  (for _array_element _outactors
    (bind _returnvalue (`self.GetDistanceTo` _array_element self))
    (if (< _returnvalue (`local.Default`))
      (set `local.Default` _returnvalue)
      (set `local.Nearest` _array_element)))
  (set `self.Control` (`local.Nearest`)))

(fn `UserConstructionScript`
  (`parent.UserConstructionScript`))