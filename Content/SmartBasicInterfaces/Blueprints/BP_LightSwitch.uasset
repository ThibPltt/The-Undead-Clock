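; BP_LightSwitch is an interactable light switch that toggles its On state and triggers its target.
; MainInteraction calls LightSwitch and plays a flashlight switch sound at the actor's location.
; LightSwitch tilts the LightSwitchBT component to one of two pitches based on the current state, then flips On.
; It then calls TurnDelayedTargetActive or TurnTargetActive, depending on HasDelay.
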(event `/Game/SmartBasicInterfaces/Blueprints/BP_MasterInteractable.MainInteraction`
  (`self.LightSwitch`)
  (`GameplayStatics.PlaySoundAtLocation` "/Game/SmartBasicInterfaces/Demo/Sounds/SC_Flashlight_Switch_Cue.SC_Flashlight_Switch_Cue" (`self.K2_GetActorLocation`) (struct) 1.0 1.0 0.0 null null null null))

(event `LightSwitch`
  (`SceneComponent.K2_SetRelativeRotation` (`self.LightSwitchBT`) (`KismetMathLibrary.MakeRotator` 0.0 (`KismetMathLibrary.SelectFloat` 5.0 -5.0 (`self.On`))) false false)
  (if (`self.On`)
    (set `self.On` false)
    (else
      (set `self.On` true)))
  (if (`self.HasDelay`)
    (`self.TurnDelayedTargetActive`)
    (else
      (`self.TurnTargetActive`))))

(fn `UserConstructionScript`
  (`parent.UserConstructionScript`))