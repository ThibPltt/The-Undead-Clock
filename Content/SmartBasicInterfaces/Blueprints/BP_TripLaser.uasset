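; BP_TripLaser is a trip-wire laser that activates its target when an actor overlaps it or its main interaction runs.
; Firing is gated by an Active flag, calls TurnTargetActive, then hides the beam cylinder, disables its collision and calls CallTripWireActive.
; PairedControlShutdown shuts down paired trip wires without triggering the target, and Reset re-arms an inactive laser by restoring visibility and collision.
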(event `self.Reset`
  (if (not (`self.Active`))
    (`SceneComponent.SetHiddenInGame` (`self.Cylinder`) false false)
    (set `self.Active` true)
    (`PrimitiveComponent.SetCollisionEnabled` (`self.Cylinder`) "QueryAndPhysics")))

(event `/Game/SmartBasicInterfaces/Blueprints/BP_MasterInteractable.MainInteraction`
  (if (`self.Active`)
    (`self.FireTripWire`)))

(event `FireTripWire`
  (if (`self.Active`)
    (`self.TurnTargetActive`)
    (`self.Deactivate`)
    (`self.TripWireActive`)))

(event `Deactivate`
  (`SceneComponent.SetHiddenInGame` (`self.Cylinder`) true false)
  (set `self.Active` false)
  (`PrimitiveComponent.SetCollisionEnabled` (`self.Cylinder`) "NoCollision"))

(event `self.ReceiveActorBeginOverlap`
  (params (OtherActor :type "Actor Object Reference"))
  (`self.FireTripWire`))

(event `self.PairedControlShutdown`
  ;[1 1 1] Deactivate Other TripWires
  (`self.Deactivate`)
  (`self.TripWireActive`))

(fn `UserConstructionScript`
  (`parent.UserConstructionScript`))