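; BP_Card is an interactable card pickup that hands its item to the actor interacting with it.
; On main interaction it sends an add-item message to the Looker with a quantity of one.
; If that succeeds, the card hides, waits briefly and destroys itself.
; Demo-only logic after the destroy call finds the level's BP_DemoPuzzleController and calls SetQ4 to update the puzzle.
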(event `self.MainInteraction`
  (bind _allow (message `/Game/SmartBasicInterfaces/Blueprints/BPI_Interactions.AddItem` (`self.Looker`) (`self.Item`) 1))
  (if _allow
    (`self.SetActorHiddenInGame` true)
    (`KismetSystemLibrary.Delay` 0.2)
    (`self.K2_DestroyActor`)
    ;[1 1 1] Only Relevant For L_Demo
    (bind _outactors (`GameplayStatics.GetAllActorsOfClass` "/Game/SmartBasicInterfaces/Blueprints/BP_DemoPuzzleController.BP_DemoPuzzleController_C"))
    (if (`KismetArrayLibrary.Array_IsNotEmpty` _outactors)
      (`/Game/SmartBasicInterfaces/Blueprints/BP_DemoPuzzleController.Set Q4` (`|GetArrayItem` _outactors)))))

(fn `UserConstructionScript`
  (`parent.UserConstructionScript`))