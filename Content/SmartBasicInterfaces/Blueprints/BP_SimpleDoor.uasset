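; BP_SimpleDoor is an interactable door that swings open and closed and can start in the open state.
; Interaction plays a sound and toggles the Open flag, calling a door control hook only when opening.
; The DoorTL timeline drives the yaw of a Rotator component, playing forward to open and in reverse to close.
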(event `self.ReceiveBeginPlay`
  (`parent.ReceiveBeginPlay`)
  (if (`self.Open`)
    (`self.OpenDoor`)))

(event `/Game/SmartBasicInterfaces/Blueprints/BP_MasterInteractable.MainInteraction`
  (`AudioComponent.Play` (`self.Audio`) 0.0)
  (if (`self.Open`)
    (`self.CloseDoor`)
    (else
      (`self.OpenDoor`)
      (`self.DoorControl`))))

(event `OpenDoor`
  (set `self.Open` true)
  (bind (_direction _newtrack_0) (`Timeline|DoorTL` :!label _label)
    (:`Update`
      (`SceneComponent.K2_SetRelativeRotation` (`self.Rotator`) (`KismetMathLibrary.MakeRotator` 0.0 0.0 _newtrack_0) false false))))

(event `CloseDoor`
  (set `self.Open` false)
  (goto _label :!via `Reverse`))

(fn `UserConstructionScript`
  (`parent.UserConstructionScript`))