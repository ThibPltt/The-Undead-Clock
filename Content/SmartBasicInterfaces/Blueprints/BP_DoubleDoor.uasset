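; BP_DoubleDoor is an interactable double door that slides two panels apart and back on alternating interactions.
; MainInteraction calls OpenDoor and plays the SCDoubledoor sound.
; A FlipFlop plays or reverses a Timeline that moves D01 and D02 along relative Y in opposite directions.
; CallDoorFullyOpen fires when the Timeline finishes with the TurnedOn flag set.
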(event `self.MainInteraction`
  (`self.OpenDoor`)
  (`AudioComponent.Play` (`self.SC_doubledoor`) 0.0))

(event `OpenDoor`
  (`/Engine/EditorBlueprintResources/StandardMacros.FlipFlop`
    (:`A`
      (set `self.TurnedOn` true)
      (bind (_direction _newtrack_0) (`Timeline|Timeline` :!label _label)
        (:`Update`
          (`SceneComponent.K2_SetRelativeLocation` (`self.D01`) (`KismetMathLibrary.MakeVector` 0.0 _newtrack_0) false false)
          (`SceneComponent.K2_SetRelativeLocation` (`self.D02`) (`KismetMathLibrary.MakeVector` 0.0 (* _newtrack_0 -1.0)) false false))
        (:`Finished`
          (if (`self.TurnedOn`)
            (`self.DoorFullyOpen`)))))
    (:`B`
      (set `self.TurnedOn` false)
      (goto _label :!via `Reverse`))))

(fn `UserConstructionScript`
  (`parent.UserConstructionScript`))