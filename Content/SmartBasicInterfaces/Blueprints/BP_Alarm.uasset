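; BP_Alarm is an alarm actor that an interaction toggles between active and silent.
; MainInteraction starts a looping timer that calls PulseLight, or clears it, zeroes the light and restores the black material.
; PulseLight uses a FlipFlop to alternate lit and dark states, switching light intensity and red emissive or black material, and playing audio on each lit pulse.
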(event `self.MainInteraction`
  (if (`self.Active`)
    (set `self.Active` false)
    (`LightComponent.SetIntensity` (`self.PointLight`) 0.0)
    (`PrimitiveComponent.SetMaterial` (`self.Alarm`) 0 "/Game/SmartBasicInterfaces/Materials/MI_BaseBlack.MI_BaseBlack")
    (`KismetSystemLibrary.K2_ClearAndInvalidateTimerHandle` (stale _returnvalue))
    (else
      (set `self.Active` true)
      (bind _returnvalue (`KismetSystemLibrary.K2_SetTimerDelegate` (delegate `PulseLight`) 0.4 true)))))

(event `PulseLight`
  (`/Engine/EditorBlueprintResources/StandardMacros.FlipFlop`
    (:`A`
      (`LightComponent.SetIntensity` (`self.PointLight`) 5000.0)
      (`PrimitiveComponent.SetMaterial` (`self.Alarm`) 0 "/Game/SmartBasicInterfaces/Materials/MI_EmissiveRed1.MI_EmissiveRed1")
      (`AudioComponent.Play` (`self.Audio`) 0.0))
    (:`B`
      (`LightComponent.SetIntensity` (`self.PointLight`) 0.0)
      (`PrimitiveComponent.SetMaterial` (`self.Alarm`) 0 "/Game/SmartBasicInterfaces/Materials/MI_BaseBlack.MI_BaseBlack"))))

(fn `UserConstructionScript`
  (`parent.UserConstructionScript`)
  (`PrimitiveComponent.CreateDynamicMaterialInstance` (`self.Alarm`) 0 "/Game/SmartBasicInterfaces/Materials/MI_BaseBlack.MI_BaseBlack" "None"))