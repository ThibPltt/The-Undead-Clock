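; Player interaction component that finds interactables, handles press and hold interactions, and keeps a weight-limited inventory.
; Each Tick it line traces from the active camera, notifying actors through BPI_Interactions when looked at or away, while MakeActive sets the current target.
; The interact input sends press or hold messages; holds run a timer with a widget, reporting success only on release.
; Items live in a quantity map, shown by the inventory widget.
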(event `/Game/SmartBasicInterfaces/Blueprints/BPI_Interactions.MakeActive`
  (params (Actor :type "Actor Object Reference"))
  (set `self.ActiveInteraction` Actor))

(event `self.ReceiveBeginPlay`
  (bind _returnvalue (pcsubsystem `EnhancedInputLocalPlayerSubsystem` (`GameplayStatics.GetPlayerController` 0)))
  (`/Engine/EditorBlueprintResources/StandardMacros.IsValid` _returnvalue
    (:`Is Valid`
      (`EnhancedInputSubsystemInterface.AddMappingContext` _returnvalue "/Game/SmartBasicInterfaces/Controls/IMC_DemoControls.IMC_DemoControls" 1 (struct)))))

(event `StopHolding`
  ;[1 1 1] Logic For Hold interaction
  (`KismetSystemLibrary.K2_ClearAndInvalidateTimerHandle` (stale `/Game/SmartBasicInterfaces/Blueprints/BPI_Interactions.MakeHoldInteraction` _returnvalue))
  (set `self.CurrentHandle` (struct))
  (bind _holdwidget (`self.HoldWidget`)
    (:`then`
      (`Widget.RemoveFromParent` _holdwidget)
      (set `self.HoldWidget` null))
    (:`else`
      _))
  (if (`self.HoldSuccess_0`)
    (message `/Game/SmartBasicInterfaces/Blueprints/BPI_Interactions.HoldSuccess` (`self.ActiveInteraction`))
    (set `self.HoldSuccess_0` false)
    (else
      (set `self.HoldSuccess_0` false))))

(event `/Game/SmartBasicInterfaces/Blueprints/BPI_Interactions.MakeHoldInteraction`
  (params (Origin :type "Actor Object Reference"))
  ;[1 1 1] Logic For Hold interaction
  (bind _asbp_master_interactable (cast `/Game/SmartBasicInterfaces/Blueprints/BP_MasterInteractable` Origin))
  (bind _returnvalue (`KismetSystemLibrary.K2_SetTimerDelegate` (delegate `HoldInteraction`) (`/Game/SmartBasicInterfaces/Blueprints/BP_MasterInteractable.HoldTime` _asbp_master_interactable)))
  (bind _output_get (set `self.CurrentHandle` _returnvalue))
  (bind _returnvalue_2 (`|CreateWidget` "/Game/SmartBasicInterfaces/Widgets/WI_HoldInteraction.WI_HoldInteraction_C" null _output_get self))
  (bind _output_get_2 (set `self.HoldWidget` _returnvalue_2))
  (`UserWidget.AddToViewport` _output_get_2 0))

(event `self.ReceiveTick`
  (params (DeltaSeconds :type "Float (single-precision)"))
  ;[1 1 1] Always Checking For Interactions
  (`|ExecutionSequence`
    (:`then_0`
      (`self.ActiveCamera`
        (:`then`
          (`self.BreakDownInteractions`))
        (:`else`)))))

(event `HoldInteraction`
  ;[1 1 1] Logic For Hold interaction
  (set `self.HoldSuccess_0` true))

(event `EnhancedInput|/Game/SmartBasicInterfaces/Controls/IA_Interact`
  (params (ActionValue :type Boolean) (ElapsedSeconds :type "Float (double-precision)") (TriggeredSeconds :type "Float (double-precision)") (InputAction :type "InputAction Object Reference" :default "/Game/SmartBasicInterfaces/Controls/IA_Interact.IA_Interact"))
  (bind _activeinteraction (`self.ActiveInteraction`))
  (bind _activeinteraction_2 (`self.ActiveInteraction`))
  (:`Started`
    (`/Engine/EditorBlueprintResources/StandardMacros.IsValid` _activeinteraction_2
      (:`Is Valid`
        (bind _type (message `/Game/SmartBasicInterfaces/Blueprints/BPI_Interactions.GetTypeOfInteraction` _activeinteraction))
        (switch `/Game/SmartBasicInterfaces/Blueprints/EN_InteractionType` _type
          (:`NewEnumerator0`
            (message `/Game/SmartBasicInterfaces/Blueprints/BPI_Interactions.Interaction01` _activeinteraction_2))
          (:`NewEnumerator1`
            (message `/Game/SmartBasicInterfaces/Blueprints/BPI_Interactions.InteractionHold` _activeinteraction))))))
  (:`Completed`
    (`self.StopHolding`)))

(event `EnhancedInput|/Game/SmartBasicInterfaces/Controls/IA_Inventory`
  (params (ActionValue :type Boolean) (ElapsedSeconds :type "Float (double-precision)") (TriggeredSeconds :type "Float (double-precision)") (InputAction :type "InputAction Object Reference" :default "/Game/SmartBasicInterfaces/Controls/IA_Inventory.IA_Inventory"))
  (:`Completed`
    (bind _returnvalue (`|CreateWidget` "/Game/SmartBasicInterfaces/Widgets/WI_Inventory.WI_Inventory_C" null self))
    (bind _output_get (set `self.InventoryWidget` _returnvalue))
    (`UserWidget.AddToViewport` _output_get 0)))

(fn `AddItem`
  (params (Item :type "/Game/SmartBasicInterfaces/Blueprints/EN_Item Enum" :default "NewEnumerator0") (Quantity :type Integer))
  (returns (Allow :type Boolean))
  (bind (_pass _totalnumber) (`/Game/SmartBasicInterfaces/Blueprints/BPL_InteractionLibrary.TransferItem` (`self.Inventory`) (`self.WeightLimit`) Item Quantity))
  (if _pass
    (`self.AddItemToInv` Item _totalnumber)
    (return true)
    (else
      (`KismetSystemLibrary.PrintString` "Over Weight Limit")
      (return false))))

(fn `AddItemToInv`
  (params (Item :type "/Game/SmartBasicInterfaces/Blueprints/EN_Item Enum" :default "NewEnumerator0") (Quantity :type Integer))
  (bind (_value _returnvalue) (`BlueprintMapLibrary.Map_Find` (`self.Inventory`) Item))
  (bind (_value_2 _returnvalue_2) (`BlueprintMapLibrary.Map_Find` (`self.Inventory`) "NewEnumerator2"))
  ;[1 1 1] Add Item to Simple Inventory
  (`BlueprintMapLibrary.Map_Add` (`self.Inventory`) Item (`KismetMathLibrary.SelectInt` (+ _value Quantity) Quantity _returnvalue))
  ;[1 1 1] Used Over the Demo Map. Can be safely Deleted
  (bind _returnvalue_3 (`GameplayStatics.GetCurrentLevelName` true))
  (if (`KismetStringLibrary.EqualEqual_StrStr` _returnvalue_3 "L_Demo")
    (if _returnvalue_2
      (if (> _value_2 1)
        (bind _outactors (`GameplayStatics.GetAllActorsOfClass` "/Game/SmartBasicInterfaces/Blueprints/BP_DemoPuzzleController.BP_DemoPuzzleController_C"))
        (`/Game/SmartBasicInterfaces/Blueprints/BP_DemoPuzzleController.Set Q8` (`|GetArrayItem` _outactors))))))

(fn `BreakDownInteractions`
  (locals (ActorHit :type "Actor Object Reference"))
  (bind _activeinteraction (`self.ActiveInteraction`))
  ;[1 1 1] Makes Interactibles active
  (set `local.ActorHit` null)
  (bind _linetracehit (`self.FindInteractions`))
  (bind (_bblockinghit _binitialoverlap _time _distance _location _impactpoint _normal _impactnormal _physmat _hitactor) (`GameplayStatics.BreakHitResult` _linetracehit))
  (bind _output_get (set `local.ActorHit` _hitactor))
  (if (not (== (`self.ActiveInteraction`) _output_get))
    (`/Engine/EditorBlueprintResources/StandardMacros.IsValid` _activeinteraction
      (:`Is Valid`
        (message `/Game/SmartBasicInterfaces/Blueprints/BPI_Interactions.StopBeingLooked` _activeinteraction self))
      (:`Is Not Valid`
        _))
    (set `self.ActiveInteraction` null)
    (if (`KismetSystemLibrary.DoesImplementInterface` _hitactor "/Game/SmartBasicInterfaces/Blueprints/BPI_Interactions.BPI_Interactions_C")
      (message `/Game/SmartBasicInterfaces/Blueprints/BPI_Interactions.BeingLookedAt` (`local.ActorHit`) self))))

(fn `FindInteractions`
  (returns (LineTraceHit :type "HitResult Structure"))
  (bind _activecamera (`self.ActiveCamera`))
  (bind _returnvalue (`SceneComponent.K2_GetComponentLocation` _activecamera))
  ;[1 1 1] LineTrace For Searching Interatctibles
  (bind _outhit (`KismetSystemLibrary.LineTraceSingle` _returnvalue (+ _returnvalue (* (`KismetMathLibrary.GetForwardVector` (`SceneComponent.K2_GetComponentRotation` _activecamera)) (`self.DistanceToInteract`))) "TraceTypeQuery1"))
  (return _outhit))

(fn `GetTypeOfInteraction`
  (returns (Type :type "/Game/SmartBasicInterfaces/Blueprints/EN_InteractionType Enum"))
  (return "NewEnumerator0"))

(fn `GiveWeightStat`
  (returns (Available :type "Float (double-precision)") (WeightLimit :type "Float (double-precision)"))
  (bind _weightlimit (`self.WeightLimit`))
  ;[1 1 1] Pass Weight stats for the library (for max weight checking)
  (bind _available (`/Game/SmartBasicInterfaces/Blueprints/BPL_InteractionLibrary.CheckTotalWeight` (`self.Inventory`) _weightlimit))
  (return _available _weightlimit))

(fn `RemoveItemFromInventory`
  (params (Item :type "/Game/SmartBasicInterfaces/Blueprints/EN_Item Enum" :default "NewEnumerator0") (Quantity :type Integer))
  (bind _value (`BlueprintMapLibrary.Map_Find` (`self.Inventory`) Item))
  ;[1 1 1] Remove Item From Simple Inventory
  (`BlueprintMapLibrary.Map_Add` (`self.Inventory`) Item (- _value Quantity))
  (if (<= _value 0)
    (`BlueprintMapLibrary.Map_Remove` (`self.Inventory`) (`local.Item`))))