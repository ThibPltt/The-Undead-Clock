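; BP_AccessPanel is an interactable access panel that takes card items from the inventory to trigger what it controls.
; Interaction runs inherited inventory checks, plays a positive sound and refreshes the visuals.
; Visibility uses the delivered item count to reveal up to two cards and swap the screen material.
; Once the requirement is met, it disables its widget and pop-up, then calls TriggerControl and CallPanelWithAllCards.
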(event `Visibility`
  (bind _delivereditens (`self.DeliveredItens`))
  (bind _plane (`self.Plane`))
  ;[1 1 1] Controls Visuals
  (`SceneComponent.SetHiddenInGame` (`self.Card01`) (select `int` _delivereditens :`0` true :`1` false :`2` false) false)
  (`SceneComponent.SetHiddenInGame` (`self.Card02`) (select `int` _delivereditens :`0` true :`1` true :`2` false) false)
  (`SceneComponent.SetHiddenInGame` _plane (not (`self.Active`)) false)
  (`PrimitiveComponent.SetMaterial` _plane 0 (select `int` _delivereditens :`0` "/Game/SmartBasicInterfaces/Materials/MI_ScreenPanel1.MI_ScreenPanel1" :`1` "/Game/SmartBasicInterfaces/Materials/MI_ScreenPanel2.MI_ScreenPanel2" :`2` "/Game/SmartBasicInterfaces/Materials/MI_ScreenPanel3.MI_ScreenPanel3" :!type "MaterialInterface Object Reference")))

(event `self.ReceiveBeginPlay`
  (`parent.ReceiveBeginPlay`)
  (`PrimitiveComponent.CreateDynamicMaterialInstance` (`self.Plane`) 0 "/Game/SmartBasicInterfaces/Materials/MI_ScreenPanel1.MI_ScreenPanel1" "None")
  (`self.Visibility`))

(event `self.ReceiveTick`
  (params (DeltaSeconds :type "Float (single-precision)"))
  (`parent.ReceiveTick` DeltaSeconds))

(event `self.MainInteraction`
  ;[1 1 1] Check For Cards
  (if (`self.HasItemRequirement?`)
    (bind _hasitem (`self.InvetoryQuickCheck`))
    (if _hasitem
      (bind _requiementmet_ (`self.InventorySearchForRequirement` true))
      (`GameplayStatics.PlaySoundAtLocation` "/Game/SmartBasicInterfaces/Demo/Sounds/SC_positive.SC_positive" (`self.K2_GetActorLocation`) (struct) 1.0 1.0 0.0 null null null null)
      (`self.Visibility`)
      (if _requiementmet_
        (set `self.HasItemRequirement?` false)
        (set `self.AllowWidget` false)
        (`SceneComponent.SetHiddenInGame` (`self.PopUP`) true false)
        (set `self.Type` "NewEnumerator0")
        (`self.TriggerControl`)
        (`self.PanelWithAllCards`)))))

(event `CardInSound`
  (`GameplayStatics.PlaySoundAtLocation` "/Game/SmartBasicInterfaces/Demo/Sounds/SC_positive.SC_positive" (`self.K2_GetActorLocation`) (struct) 1.0 1.0 0.0 null null null null))

(fn `UserConstructionScript`
  (`parent.UserConstructionScript`))