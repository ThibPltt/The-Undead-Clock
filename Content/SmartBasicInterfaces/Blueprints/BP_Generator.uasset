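; Interactable generator that needs an inventory item, apparently fuel, before it can be switched on and off.
; While the requirement stands, interaction searches the inventory, plays a pouring sound and, on success, clears the requirement, hides the popup and fires HasFuel.
; Later interactions toggle power and fire GeneratorOn either way.
; A timeline plays or reverses with power, driving material glow and clamped audio volume.
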(event `self.MainInteraction`
  (if (`self.HasItemRequirement?`)
    ;[1 1 1] Check And Fill Generator
    (bind _hasitem (`self.InvetoryQuickCheck`))
    (if _hasitem
      (bind _requiementmet_ (`self.InventorySearchForRequirement` true))
      (`GameplayStatics.PlaySoundAtLocation` "/Game/SmartBasicInterfaces/Sound/SC_gaspour.SC_gaspour" (`self.K2_GetActorLocation`) (struct) 1.0 1.0 0.0 null null null null)
      (if _requiementmet_
        (set `self.FreeFromControls` false)
        (set `self.HasItemRequirement?` false)
        (set `self.AllowWidget` false)
        (`SceneComponent.SetHiddenInGame` (`self.PopUP`) true false)
        (`self.HasFuel`)))
    (else
      (`self.On/Off` (not (`self.TurnedOn`)))
      (`self.GeneratorOn`))))

(event `On/Off`
  (params (On :type Boolean))
  (bind _output_get (set `self.TurnedOn` On))
  (if _output_get
    (bind (_direction _newtrack_0) (`Timeline|Timeline` :!label _label)
      (:`Update`
        (`MeshComponent.SetScalarParameterValueOnMaterials` (`self.Front`) "Glow" _newtrack_0)
        (`MeshComponent.SetScalarParameterValueOnMaterials` (`self.Section1`) "Glow" _newtrack_0)
        (`MeshComponent.SetScalarParameterValueOnMaterials` (`self.Section2`) "Glow" _newtrack_0)
        (`MeshComponent.SetScalarParameterValueOnMaterials` (`self.Section3`) "Glow" _newtrack_0)
        (`AudioComponent.SetVolumeMultiplier` (`self.Audio`) (`KismetMathLibrary.FClamp` (* _newtrack_0 0.4) 0.01 2.0))))
    (else
      (goto _label :!via `Reverse`))))

(fn `UserConstructionScript`
  (`parent.UserConstructionScript`))