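; Blueprint function library that checks whether a receiving inventory has weight capacity for an item transfer.
; TransferItem feeds the remaining capacity from CheckTotalWeight into CheckWeightForTransfer, returning a pass flag and the quantity that fits, without modifying the inventory.
; Inventories map item enums to quantities, with unit weights looked up in DT_ItemList by enum name.
; Oversized requests are truncated to whole units that fit, failing when not even one fits.
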(fn `CheckTotalWeight`
  (params (Inventory :type "Map of /Game/SmartBasicInterfaces/Blueprints/EN_Item Enum to Integer") (Limit :type "Float (double-precision)"))
  (returns (Available :type "Float (double-precision)"))
  (locals (TotalWeight :type "Float (double-precision)"))
  ;[1 1 1] Find the total and available weight for target inventory
  (set `local.TotalWeight` 0.0)
  (bind _keys (`BlueprintMapLibrary.Map_Keys` Inventory))
  (for _array_element _keys
    (bind _returnvalue (`|GetDataTableRow` "/Game/SmartBasicInterfaces/Blueprints/DT_ItemList.DT_ItemList" (`KismetStringLibrary.Conv_StringToName` (`|GetEnumeratorNameAsString` _array_element)))
      (:`then`
        (set `local.TotalWeight` (+ (`local.TotalWeight`) (* (`BlueprintMapLibrary.Map_Find` Inventory _array_element) (`.Weight_5_221041784FB09DCECB7BB5AFF585E0EC` (break `/Game/SmartBasicInterfaces/Blueprints/ST_Item` _returnvalue))))))))
  (return (- (`local.Limit`) (`local.TotalWeight`))))

(fn `CheckWeightForTransfer`
  (params (Item :type "/Game/SmartBasicInterfaces/Blueprints/EN_Item Enum" :default "NewEnumerator0") (Quantity :type Integer) (Limit :type "Float (double-precision)"))
  (returns (Pass :type Boolean) (TotalNumber :type Integer))
  ;[1 1 1] See If there is Room on target inventory
  (bind _returnvalue (`|GetDataTableRow` "/Game/SmartBasicInterfaces/Blueprints/DT_ItemList.DT_ItemList" (`KismetStringLibrary.Conv_StringToName` (`|GetEnumeratorNameAsString` Item)))
    (:`then`
      (bind (_item _weight) (break `/Game/SmartBasicInterfaces/Blueprints/ST_Item` _returnvalue))
      (if (<= (* _weight (`local.Quantity`)) (`local.Limit`))
        (return true (`local.Quantity`))
        (else
          (bind _returnvalue_2 (/ (`local.Limit`) _weight))
          (if (< _returnvalue_2 1.0)
            (return false 0)
            (else
              (return true (`KismetMathLibrary.FTrunc` _returnvalue_2)))))))))

(fn `TransferItem`
  (params (Receiver :type "Map of /Game/SmartBasicInterfaces/Blueprints/EN_Item Enum to Integer") (Limit :type "Float (double-precision)") (Item :type "/Game/SmartBasicInterfaces/Blueprints/EN_Item Enum" :default "NewEnumerator0") (Quantity :type Integer))
  (returns (Pass :type Boolean) (TotalNumber :type Integer))
  ;[1 1 1] Transfer Item Function (checks space for item and clear it or not)
  (bind _available (`self.CheckTotalWeight` Receiver Limit))
  (bind (_pass _totalnumber) (`self.CheckWeightForTransfer` Item Quantity _available))
  (return _pass _totalnumber))