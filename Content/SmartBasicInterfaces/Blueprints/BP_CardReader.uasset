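; BP_CardReader is an interactable card reader that checks the inventory on interaction.
; A successful search calls TriggerControl and plays a positive sound, while failure prints a missing-card error and plays a negative sound.
; Both results blink the Reader's emissive color green or red through a looping timer and DoN counter, which stops the timer and restores white.
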(event `StopBlink`
  ;[1 1 1] Light Blinking
  (`KismetSystemLibrary.K2_ClearAndInvalidateTimerHandle` (stale `QuickLightBlink` _returnvalue))
  (`MeshComponent.SetVectorParameterValueOnMaterials` (`self.Reader`) "EmissiveColor" (`KismetMathLibrary.Conv_LinearColorToVector` (struct :`R` 1.0 :`G` 1.0 :`B` 1.0 :`A` 1.0))))

(event `QuickLightBlink`
  (params (Pass :type Boolean))
  ;[1 1 1] Light Blinking
  (`|ExecutionSequence`
    (:`then_0`
      (bind _returnvalue (`KismetSystemLibrary.K2_SetTimerDelegate` (delegate `Blink`) 0.2 true)))
    (:`then_1`
      (goto _label :!via `Reset`))))

(event `Blink`
  ;[1 1 1] Light Blinking
  (bind _counter (`/Engine/EditorBlueprintResources/StandardMacros.Do N` 6 :!label _label)
    (:`Exit`
      (if (>= _counter 6)
        (`self.StopBlink`)
        (else
          (`MeshComponent.SetVectorParameterValueOnMaterials` (`self.Reader`) "EmissiveColor" (`KismetMathLibrary.Conv_LinearColorToVector` (`KismetMathLibrary.SelectColor` (struct :`G` 1.0 :`B` 0.15713 :`A` 1.0) (struct :`R` 1.0 :`B` 0.016184 :`A` 1.0) (stale `QuickLightBlink` Pass))))
          (`KismetSystemLibrary.Delay` 0.1)
          (`MeshComponent.SetVectorParameterValueOnMaterials` (`self.Reader`) "EmissiveColor" (`KismetMathLibrary.Conv_LinearColorToVector` (struct :`R` 1.0 :`G` 1.0 :`B` 1.0 :`A` 1.0))))))))

(event `self.MainInteraction`
  (bind _found (`self.InventorySearchSimple` false))
  (if _found
    (`self.TriggerControl`)
    (`self.QuickLightBlink` true)
    (`GameplayStatics.PlaySoundAtLocation` "/Game/SmartBasicInterfaces/Demo/Sounds/SC_positive.SC_positive" (`self.K2_GetActorLocation`) (struct) 1.0 1.0 0.0 null null null null)
    (else
      (`KismetSystemLibrary.PrintString` "ERROR - NO CARD")
      (`self.QuickLightBlink` false)
      (`GameplayStatics.PlaySoundAtLocation` "/Game/SmartBasicInterfaces/Demo/Sounds/SC_negative.SC_negative" (`self.K2_GetActorLocation`) (struct) 1.0 1.0 0.0 null null null null))))

(fn `UserConstructionScript`
  (`parent.UserConstructionScript`))