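; BP_PowerBTN is an interactable power button that reacts to the main interaction by playing a push sound and animating a press.
; It sets a cooldown flag, then a timeline moves the button mesh along its local X axis.
; When the animation finishes, it triggers its controlled target and fires a button-pressed call, building on a parent interface Blueprint.
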(event `self.MainInteraction`
  (`self.BTNAction`))

(event `BTNAction`
  (`GameplayStatics.PlaySoundAtLocation` "/Game/Environment/SmartBasicInterfaces/Sound/SC_button-push.SC_button-push" (`self.K2_GetActorLocation`) (struct) 1.0 1.0 0.0 null null null null)
  (set `self.OnCoolDown` true)
  (`self.Press`))

(event `Press`
  (bind (_direction _newtrack_0) (`Timeline|Timeline` :!via `PlayFromStart`)
    (:`Update`
      (`SceneComponent.K2_SetRelativeLocation` (`self.BTN`) (`KismetMathLibrary.MakeVector` _newtrack_0) false false))
    (:`Finished`
      (`self.TriggerControl`)
      (`self.ButtonPressed`))))

(fn `UserConstructionScript`
  (`parent.UserConstructionScript`))