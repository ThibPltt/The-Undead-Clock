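; Base interactable target that handles press and hold interactions and can optionally carry an inventory stash, added as an AC_Stash component at BeginPlay.
; Both inputs pass active, control, optional fire-once and required-item checks, with the DoOnce consumed before the item check until Reset.
; Press calls MainInteraction directly, while hold messages the Looker and runs MainInteraction on HoldSuccess.
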(event `self.ReceiveBeginPlay`
  (`parent.ReceiveBeginPlay`)
  ;[1 1 1] Check for creating AC_Stash
  (`self.StashCheck`))

(event `/Game/Environment/SmartBasicInterfaces/Blueprints/BPI_Interactions.Interaction01`
  ;[1 1 1] Interface for "Press"
  (if (`self.Active`)
    (if (`self.FreeFromControls`)
      (if (`self.FiresOnce`)
        (`/Engine/EditorBlueprintResources/StandardMacros.DoOnce` false :!label _label
          (:`Completed`
            _)))
      (if (`self.HasItemRequirement?`)
        (bind _hasitem (`self.InvetoryQuickCheck`))
        (if _hasitem
          (`self.MainInteraction` :!label _label_2))
        (else
          (goto _label_2))))))

(event `Reset`
  ;[1 1 1] Call for reseting "Fire Once"
  (`|ExecutionSequence`
    (:`then_0`
      (goto _label :!via `Reset`))
    (:`then_1`
      (goto _label_3 :!via `Reset`))))

(event `/Game/Environment/SmartBasicInterfaces/Blueprints/BPI_Interactions.InteractionHold`
  ;[1 1 1] Interface for "Hold"
  (if (`self.Active`)
    (if (`self.FreeFromControls`)
      (if (`self.FiresOnce`)
        (`/Engine/EditorBlueprintResources/StandardMacros.DoOnce` false :!label _label_3
          (:`Completed`
            _)))
      (if (`self.HasItemRequirement?`)
        (bind _hasitem (`self.InvetoryQuickCheck`))
        (if _hasitem
          (message `/Game/Environment/SmartBasicInterfaces/Blueprints/BPI_Interactions.MakeHoldInteraction` (`self.Looker`) self :!label _label_4))
        (else
          (goto _label_4))))))

(event `/Game/Environment/SmartBasicInterfaces/Blueprints/BPI_Interactions.HoldSuccess`
  (`self.MainInteraction`))

(fn `StashCheck`
  ;[1 1 1] Adds AC_Stash actor component
  (if (`self.HasStash`)
    (bind _returnvalue (`AddComponent|NODE_AddACStash-1` :`StashInventory` (`self.Stash`) :`WeightLimit` (`self.Weight Limit`)))
    (set `self.StashRef` _returnvalue)))

(fn `UserConstructionScript`
  (`parent.UserConstructionScript`))