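; Interactable control that activates a list of target Controls through press or hold interactions, with active, fire-once, inventory item and press cooldown checks.
; Hold input asks the Looker to show a hold interaction, and its success runs MainInteraction.
; TriggerControl fires targets immediately, all after one delay, or one by one on a looping timer.
; Simultaneous firing also calls PairedControlShutdown, an empty hook here, on other fire-once paired controls.
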(event `TriggerControl`
  ;[1 1 1] Trigger Control -> Controls to Targets
  (if (`self.HasDelay`)
    (`self.TurnDelayedTargetActive`)
    (else
      (`self.TurnTargetActive`))))

(event `PairedControlShutdown`
  ;[1 1 1] Event for paired shutdowns
)

(event `TurnTargetActive`
  ;[1 1 1] Activates The Target
  (for _array_element (`self.Controls`)
    (`self.MainInteraction` _array_element))
  ;[1 1 1] For Shutdowns of paired Controls
  (set `self.OnCoolDown` false)
  (if (> (`KismetArrayLibrary.Array_Length` (`self.PairedControls`)) 0)
    (for _array_element_2 (`self.PairedControls`)
      (if (!= _array_element_2 self)
        (if (`/Game/Environment/SmartBasicInterfaces/Blueprints/BP_MasterControl.FiresOnce` _array_element_2)
          (`self.PairedControlShutdown` _array_element_2))))))

(event `/Game/Environment/SmartBasicInterfaces/Blueprints/BPI_Interactions.Interaction01`
  ;[1 1 1] Interface for the "Press" Interaction
  (if (`self.Active`)
    (if (`self.FiresOnce`)
      (`/Engine/EditorBlueprintResources/StandardMacros.DoOnce` false :!label _label
        (:`Completed`
          _)))
    (if (`self.HasItemRequirement?`)
      (bind _hasitem (`self.InvetoryQuickCheck`))
      (if _hasitem
        (if (`self.OnCoolDown`) :!label _label_2
          (`self.CoolDown`)
          (else
            (`self.MainInteraction`))))
      (else
        (goto _label_2)))))

(event `Reset`
  ;[1 1 1] Call this event to reset Fire Once Actor
  (`|ExecutionSequence`
    (:`then_0`
      (goto _label :!via `Reset`))
    (:`then_1`
      (goto _label_3 :!via `Reset`))))

(event `TurnDelayedTargetActive`
  ;[1 1 1] Simple Delay
  (if (`self.AllTargetsWithDelay`)
    ;[1 1 1] For multiple Delays
    (bind _returnvalue (`KismetSystemLibrary.K2_SetTimerDelegate` (delegate `SendSignal`) (`self.Delay`) (> (`KismetArrayLibrary.Array_Length` (`self.Controls`)) 1)))
    (set `self.DelayTH` _returnvalue)
    (else
      (bind _returnvalue_2 (`KismetSystemLibrary.K2_SetTimerDelegate` (delegate `TurnTargetActive`) (`self.Delay`)))
      (set `self.DelayTH` _returnvalue_2))))

(event `/Game/Environment/SmartBasicInterfaces/Blueprints/BPI_Interactions.InteractionHold`
  ;[1 1 1] Interface for "Hold"
  (if (`self.Active`)
    (if (`self.FiresOnce`)
      (`/Engine/EditorBlueprintResources/StandardMacros.DoOnce` false :!label _label_3
        (:`Completed`
          _)))
    (if (`self.HasItemRequirement?`)
      (bind _hasitem (`self.InvetoryQuickCheck`))
      (if _hasitem
        (message `/Game/Environment/SmartBasicInterfaces/Blueprints/BPI_Interactions.MakeHoldInteraction` (`self.Looker`) self :!label _label_4))
      (else
        (goto _label_4)))))

(event `/Game/Environment/SmartBasicInterfaces/Blueprints/BPI_Interactions.HoldSuccess`
  ;[1 1 1] Interface for "Hold"
  (`self.MainInteraction`))

(event `SendSignal`
  (bind _controls (`self.Controls`))
  ;[1 1 1] For multiple Delays
  (`self.MainInteraction` (`|GetArrayItem` _controls (`self.DelayedCount`)))
  (bind _result (`/Engine/EditorBlueprintResources/StandardMacros.IncrementInt` (`self.DelayedCount`))
    (:`  `
      (if (>= _result (`KismetArrayLibrary.Array_Length` _controls))
        (set `self.OnCoolDown` false)
        (set `self.DelayedCount` 0)
        (`KismetSystemLibrary.K2_ClearAndInvalidateTimerHandle` (stale `TurnDelayedTargetActive` _returnvalue))))))

(fn `UserConstructionScript`
  (`parent.UserConstructionScript`))