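; BP_Lever is an interactable lever that toggles between on and off, playing a sound and triggering a control action.
; MainInteraction calls Activate, which flips TurnedOn and runs one timeline forward or in reverse to rotate the lever's pitch.
; OnCoolDown is set during the swing; on finish, TriggerControl fires and the cooldown clears.
; BeginPlay also runs Activate, with FirstActivation intended to suppress that initial trigger.
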(event `self.MainInteraction`
  (`self.Activate`))

(event `Activate`
  (`AudioComponent.Play` (`self.Audio`) 0.0)
  (if (`self.TurnedOn`)
    (`self.LeverDown`)
    (else
      (`self.LeverUp`))))

(event `self.ReceiveBeginPlay`
  (`parent.ReceiveBeginPlay`)
  (`self.Activate`))

(event `self.ReceiveTick`
  (params (DeltaSeconds :type "Float (single-precision)"))
  (`parent.ReceiveTick` DeltaSeconds))

(event `LeverUp`
  (set `self.OnCoolDown` true)
  (set `self.TurnedOn` true)
  (bind (_direction _newtrack_0) (`Timeline|TimelineAction` :!via `Reverse` :!label _label)
    (:`Update`
      (`SceneComponent.K2_SetRelativeRotation` (`self.Lever_Movable`) (`KismetMathLibrary.MakeRotator` 0.0 _newtrack_0) false false))
    (:`Finished`
      (`|ExecutionSequence`
        (:`then_0`
          (if (not (`self.FirstActivation`))
            (`self.TriggerControl`)))
        (:`then_1`
          (`/Engine/EditorBlueprintResources/StandardMacros.DoOnce` false
            (:`Completed`
              (set `self.FirstActivation` false))))
        (:`then_2`
          (set `self.OnCoolDown` false))))))

(event `LeverDown`
  (set `self.OnCoolDown` true)
  (set `self.TurnedOn` false)
  (goto _label))

(fn `UserConstructionScript`
  (`parent.UserConstructionScript`))