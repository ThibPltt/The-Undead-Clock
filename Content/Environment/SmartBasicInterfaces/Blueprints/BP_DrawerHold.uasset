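; BP_DrawerHold is an interactable drawer that gives the player access to a stash through an item transfer screen.
; Its MainInteraction event plays the open and search sounds at the actor's location in the same sequence, setting the Type enum once via DoOnce.
; Each interaction also creates a WI_ItemTransfer widget, passing it Looker and StashRef, and adds it to the viewport.
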(event `self.ReceiveBeginPlay`
  (`parent.ReceiveBeginPlay`))

(event `self.MainInteraction`
  (bind _returnvalue (`self.K2_GetActorLocation`))
  (`|ExecutionSequence`
    (:`then_0`
      (`GameplayStatics.PlaySoundAtLocation` "/Game/Environment/SmartBasicInterfaces/Sound/SC_draweropen.SC_draweropen" _returnvalue (struct) 1.0 1.0 0.0 null null null null)
      (`/Engine/EditorBlueprintResources/StandardMacros.DoOnce` false
        (:`Completed`
          (set `self.Type` "NewEnumerator0"))))
    (:`then_1`
      (`GameplayStatics.PlaySoundAtLocation` "/Game/Environment/SmartBasicInterfaces/Sound/SC_drawersearch.SC_drawersearch" _returnvalue (struct) 1.0 1.0 0.0 null null null null)
      (bind _returnvalue_2 (`|CreateWidget` "/Game/Environment/SmartBasicInterfaces/Widgets/WI_ItemTransfer.WI_ItemTransfer_C" null (`self.Looker`) (`self.StashRef`)))
      (`UserWidget.AddToViewport` _returnvalue_2 0))))

(fn `UserConstructionScript`
  (`parent.UserConstructionScript`))