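; BP_Drawer is an interactable drawer that slides open and closed and can hold a pickup card.
; BeginPlay places the Drawer component according to the Closed flag.
; MainInteraction plays audio and toggles Open or Close, which run one Timeline forward or in reverse to drive the drawer's relative X position.
; SpawnCardInside spawns a BP_Card at Spawn01 and attaches it to the Drawer component, keeping its world transform.
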(event `self.ReceiveBeginPlay`
  (`parent.ReceiveBeginPlay`)
  (`SceneComponent.K2_SetRelativeLocation` (`self.Drawer`) (`KismetMathLibrary.MakeVector` (`KismetMathLibrary.SelectFloat` 0.0 40.0 (`self.Closed`))) false false))

(event `/Game/Environment/SmartBasicInterfaces/Blueprints/BP_MasterInteractable.MainInteraction`
  (`AudioComponent.Play` (`self.Audio`) 0.0)
  (if (`self.Closed`)
    (`self.Open`)
    (else
      (`self.Close`))))

(event `Open`
  (set `self.Closed` false)
  (bind (_direction _newtrack_0) (`Timeline|Timeline` :!label _label)
    (:`Update`
      (`SceneComponent.K2_SetRelativeLocation` (`self.Drawer`) (`KismetMathLibrary.MakeVector` _newtrack_0) false false))))

(event `Close`
  (set `self.Closed` true)
  (goto _label :!via `Reverse`))

(event `SpawnCardInside`
  (bind _returnvalue (`|SpawnActorFromClass` "/Game/Environment/SmartBasicInterfaces/Blueprints/BP_Card.BP_Card_C" (`SceneComponent.K2_GetComponentToWorld` (`self.Spawn01`)) "AlwaysSpawn" "OverrideRootScale" null true true false 15.0 "Pick Up" true "NewEnumerator0" 0.0 1 "NewEnumerator0" false true null))
  (`self.K2_AttachToComponent` _returnvalue (`self.Drawer`) "None" "KeepWorld" "KeepWorld" "KeepWorld" false))

(fn `UserConstructionScript`
  (`parent.UserConstructionScript`))