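; Demo first-person player for the Smart Basic Interfaces environment, with a battery-powered flashlight, demo HUD and pause menu.
; BeginPlay hands the first-person camera to the ACPlayerInteractions component, which also holds the inventory.
; The flashlight toggle runs a looping timer that drains charge, then consumes an inventory battery to refill, or switches off if none remain.
; AddItem and GetTypeOfInteraction return only fixed values.
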(event `AssignCameraToInteractionComponent`
  (params (ActiveCamera :type "CameraComponent Object Reference"))
  ;[0.007625 1 0.1571] Basic Setup
  ;;[1 1 1] Pass The Camera Information To The Component
  (set `/Game/Environment/SmartBasicInterfaces/Blueprints/AC_PlayerInteractions.ActiveCamera` ActiveCamera (`self.AC_PlayerInteractions`)))

(event `self.ReceiveBeginPlay`
  (`parent.ReceiveBeginPlay`)
  ;[0.007625 1 0.1571] Basic Setup
  ;;[1 1 1] Setup For The Interaction System
  (`self.AssignCameraToInteractionComponent` (`self.FirstPersonCamera`))
  ;[1 1 1] DemoWidget
  (bind _returnvalue (`|CreateWidget` "/Game/Environment/SmartBasicInterfaces/Widgets/WI_DemoHUD.WI_DemoHUD_C" null self))
  (`UserWidget.AddToViewport` _returnvalue 0))

(event `EnhancedInput|/Game/Environment/SmartBasicInterfaces/Controls/IA_FlashLight`
  (params (ActionValue :type Boolean) (ElapsedSeconds :type "Float (double-precision)") (TriggeredSeconds :type "Float (double-precision)") (InputAction :type "InputAction Object Reference" :default "/Game/Environment/SmartBasicInterfaces/Controls/IA_FlashLight.IA_FlashLight"))
  ;[1 1 1] FlashLight Controls
  (:`Completed`
    (if (> (`self.FlashLightBattery`) 0.0)
      (if (`self.FlashLightOn`)
        (`self.TurnFlashLightOff`)
        (else
          (`self.TurnFlashLightON`)))
      (else
        (`self.UseABattery`)))))

(event `FlashLightConsumeOff`
  ;[1 1 1] FlashLightBattery consumption
  (`KismetSystemLibrary.K2_ClearAndInvalidateTimerHandle` (stale `FlashLightConsume` _returnvalue)))

(event `TurnFlashLightOff`
  ;[1 1 1] FlashLight Controls
  (`GameplayStatics.PlaySound2D` "/Game/Environment/SmartBasicInterfaces/Demo/Sounds/SW_Flashlight_Switch.SW_Flashlight_Switch" 1.0 1.0 0.0 null null)
  (`LightComponent.SetIntensity` (`self.SpotLight`) 0.0)
  (set `self.FlashLightOn` false)
  (`self.FlashLightConsumeOff`))

(event `FlashLightConsume`
  ;[1 1 1] FlashLightBattery consumption
  (bind _returnvalue (`KismetSystemLibrary.K2_SetTimerDelegate` (delegate `ConsumeBattery`) 0.1 true)))

(event `TurnFlashLightON`
  ;[1 1 1] FlashLight Controls
  (`GameplayStatics.PlaySound2D` "/Game/Environment/SmartBasicInterfaces/Demo/Sounds/SW_Flashlight_Switch.SW_Flashlight_Switch" 1.0 1.0 0.0 null null)
  (`LightComponent.SetIntensity` (`self.SpotLight`) 1500.0)
  (set `self.FlashLightOn` true)
  (`self.FlashLightConsume`))

(event `ConsumeBattery`
  ;[1 1 1] FlashLightBattery consumption
  (`/Engine/EditorBlueprintResources/StandardMacros.DecrementFloat` (`self.FlashLightBattery`)
    (:`  `
      (if (< (`self.FlashLightBattery`) 0.0)
        (`self.UseABattery`)))))

(event `EnhancedInput|/Game/Environment/SmartBasicInterfaces/Controls/IA_Pause`
  (params (ActionValue :type Boolean) (ElapsedSeconds :type "Float (double-precision)") (TriggeredSeconds :type "Float (double-precision)") (InputAction :type "InputAction Object Reference" :default "/Game/Environment/SmartBasicInterfaces/Controls/IA_Pause.IA_Pause"))
  (:`Started`
    (bind _returnvalue (`|CreateWidget` "/Game/Environment/SmartBasicInterfaces/Widgets/WI_Pause.WI_Pause_C"))
    (`UserWidget.AddToViewport` _returnvalue 0)))

(fn `AddItem`
  (params (Item :type "/Game/Environment/SmartBasicInterfaces/Blueprints/EN_Item Enum" :default "NewEnumerator0") (Quantity :type Integer))
  (returns (Allow :type Boolean))
  (return false))

(fn `GetTypeOfInteraction`
  (returns (Type :type "/Game/Environment/SmartBasicInterfaces/Blueprints/EN_InteractionType Enum"))
  (return "NewEnumerator0"))

(fn `UseABattery`
  (bind (_value _returnvalue) (`BlueprintMapLibrary.Map_Find` (`/Game/Environment/SmartBasicInterfaces/Blueprints/AC_PlayerInteractions.Inventory` (`self.AC_PlayerInteractions`)) "NewEnumerator3"))
  ;[1 1 1] Checks For Battery at the inventory and consumes if found
  (if (and _returnvalue (> _value 0))
    (set `self.FlashLightBattery` (`self.FlashLightBatteryMax`))
    (`/Game/Environment/SmartBasicInterfaces/Blueprints/AC_PlayerInteractions.RemoveItemFromInventory` (`self.AC_PlayerInteractions`) "NewEnumerator3" 1)
    (if (not (`self.FlashLightOn`))
      (`self.TurnFlashLightON`))
    (else
      (`self.TurnFlashLightOff`))))

(fn `UserConstructionScript`
  (`parent.UserConstructionScript`))