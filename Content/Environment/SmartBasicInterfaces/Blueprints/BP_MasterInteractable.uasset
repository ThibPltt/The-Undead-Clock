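; Base Blueprint for interactable objects, with empty interaction, hold-success and cooldown events, presumably for children to implement.
; Being looked at stores the Looker, notifies it and shows the pop-up widget if allowed; looking away stops holding, clears it and hides the widget.
; Helper functions check the Looker's inventory for a required item and can remove it, either all at once or incrementally, tracking delivered progress.
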(event `self.ReceiveBeginPlay`
  (`self.PopUpWidgetCreation`))

(event `/Game/Environment/SmartBasicInterfaces/Blueprints/BPI_Interactions.Interaction01`)

(event `MainInteraction`)

(event `CoolDown`)

(event `/Game/Environment/SmartBasicInterfaces/Blueprints/BPI_Interactions.InteractionHold`)

(event `/Game/Environment/SmartBasicInterfaces/Blueprints/BPI_Interactions.BeingLookedAt`
  (params (Looker :type "/Game/Environment/SmartBasicInterfaces/Blueprints/AC_PlayerInteractions Object Reference"))
  (if (`self.AllowWidget`)
    (`self.Show/HideWidget` false))
  (message `/Game/Environment/SmartBasicInterfaces/Blueprints/BPI_Interactions.MakeActive` Looker self)
  (set `self.Looker` Looker))

(event `/Game/Environment/SmartBasicInterfaces/Blueprints/BPI_Interactions.StopBeingLooked`
  (params (Looker :type "/Game/Environment/SmartBasicInterfaces/Blueprints/AC_PlayerInteractions Object Reference"))
  (`/Game/Environment/SmartBasicInterfaces/Blueprints/AC_PlayerInteractions.StopHolding` Looker)
  (set `self.Looker` null)
  (`self.Show/HideWidget` true))

(event `/Game/Environment/SmartBasicInterfaces/Blueprints/BPI_Interactions.HoldSuccess`)

(fn `AddItem`
  (params (Item :type "/Game/Environment/SmartBasicInterfaces/Blueprints/EN_Item Enum" :default "NewEnumerator0") (Quantity :type Integer))
  (returns (Allow :type Boolean))
  (return false))

(fn `GetTypeOfInteraction`
  (returns (Type :type "/Game/Environment/SmartBasicInterfaces/Blueprints/EN_InteractionType Enum"))
  (return (`self.Type`)))

(fn `InventorySearchForRequirement`
  (params (`RemoveItens?` :type Boolean))
  (returns (`RequiementMet?` :type Boolean))
  (locals (TotalItensOfInterest :type Integer) (Delivering :type Integer))
  (set `local.TotalItensOfInterest` 0)
  (set `local.TotalItensOfInterest` (`BlueprintMapLibrary.Map_Find` (`/Game/Environment/SmartBasicInterfaces/Blueprints/AC_PlayerInteractions.Inventory` (`self.Looker`)) (`self.ItemToLookFor`)))
  (if (`self.AllItemsAtOnce`)
    (bind _output_get (set `local.Delivering` (`KismetMathLibrary.SelectInt` (- (`self.ItemQuantityToLookFor`) (`self.DeliveredItens`)) (`local.TotalItensOfInterest`) (>= (`local.TotalItensOfInterest`) (- (`self.ItemQuantityToLookFor`) (`self.DeliveredItens`))))))
    (`/Game/Environment/SmartBasicInterfaces/Blueprints/AC_PlayerInteractions.RemoveItemFromInventory` (`self.Looker`) (`self.ItemToLookFor`) _output_get)
    (set `self.DeliveredItens` (+ (`self.DeliveredItens`) (`local.Delivering`)))
    (else
      (`/Game/Environment/SmartBasicInterfaces/Blueprints/AC_PlayerInteractions.RemoveItemFromInventory` (`self.Looker`) (`self.ItemToLookFor`) 1)
      (`/Engine/EditorBlueprintResources/StandardMacros.IncrementInt` (`self.DeliveredItens`)
        (:`  `
          _))))
  (return (>= (`self.DeliveredItens`) (`self.ItemQuantityToLookFor`))))

(fn `InventorySearchSimple`
  (params (`RemoveItens?` :type Boolean))
  (returns (Found :type Boolean))
  (bind (_value _returnvalue) (`BlueprintMapLibrary.Map_Find` (`/Game/Environment/SmartBasicInterfaces/Blueprints/AC_PlayerInteractions.Inventory` (`self.Looker`)) (`self.ItemToLookFor`)))
  (if _returnvalue
    (if (>= _value (`self.ItemQuantityToLookFor`))
      (if `RemoveItens?`
        (`/Game/Environment/SmartBasicInterfaces/Blueprints/AC_PlayerInteractions.RemoveItemFromInventory` (`self.Looker`) (`self.ItemToLookFor`) (`self.ItemQuantityToLookFor`)))
      (return true)
      (else
        _)))
  (return false))

(fn `InvetoryQuickCheck`
  (returns (HasItem :type Boolean))
  (bind (_value _returnvalue) (`BlueprintMapLibrary.Map_Find` (`/Game/Environment/SmartBasicInterfaces/Blueprints/AC_PlayerInteractions.Inventory` (`self.Looker`)) (`self.ItemToLookFor`)))
  (`self.Looker`
    (:`then`
      (return (and _returnvalue (> _value 0))))
    (:`else`
      (return false))))

(fn `PopUpWidgetCreation`
  (bind _aswi_pop_up (cast `/Game/Environment/SmartBasicInterfaces/Widgets/WI_PopUp` (`WidgetComponent.GetUserWidgetObject` (`self.PopUP`))))
  (set `/Game/Environment/SmartBasicInterfaces/Widgets/WI_PopUp.PopUPTEXT` (`self.Pop UPTEXT`) _aswi_pop_up))

(fn `Show/HideWidget`
  (params (Hide :type Boolean))
  (`SceneComponent.SetHiddenInGame` (`self.PopUP`) Hide false))

(fn `UserConstructionScript`)