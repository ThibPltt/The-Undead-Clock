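; ACStash is a stash inventory component that stores items with their quantities in a map and tracks them against a weight limit.
; Adding an item increases its existing count or creates the entry, while removing subtracts the quantity and deletes entries that reach zero or below.
; GiveWeightStat passes the map and limit to CheckTotalWeight and returns the result as Available alongside the limit.
; Neither add nor remove checks the weight limit.
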(fn `AddItemToInv`
  (params (Item :type "/Game/Environment/SmartBasicInterfaces/Blueprints/EN_Item Enum" :default "NewEnumerator0") (Quantity :type Integer))
  (bind (_value _returnvalue) (`BlueprintMapLibrary.Map_Find` (`self.StashInventory`) Item))
  (`BlueprintMapLibrary.Map_Add` (`self.StashInventory`) Item (`KismetMathLibrary.SelectInt` (+ _value Quantity) Quantity _returnvalue)))

(fn `GiveWeightStat`
  (returns (Available :type "Float (double-precision)") (WeightLimit :type "Float (double-precision)"))
  (bind _weightlimit (`self.WeightLimit`))
  (bind _available (`/Game/Environment/SmartBasicInterfaces/Blueprints/BPL_InteractionLibrary.CheckTotalWeight` (`self.StashInventory`) _weightlimit))
  (return _available _weightlimit))

(fn `RemoveItemFromInventory`
  (params (Item :type "/Game/Environment/SmartBasicInterfaces/Blueprints/EN_Item Enum" :default "NewEnumerator0") (Quantity :type Integer))
  (bind _value (`BlueprintMapLibrary.Map_Find` (`self.StashInventory`) Item))
  (`BlueprintMapLibrary.Map_Add` (`self.StashInventory`) Item (- _value Quantity))
  (if (<= _value 0)
    (`BlueprintMapLibrary.Map_Remove` (`self.StashInventory`) (`local.Item`))))